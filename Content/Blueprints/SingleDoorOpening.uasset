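; A single swinging door Blueprint that toggles between open and closed when DoorOrderAction is called, ignoring calls while it is moving.
; Tick rotates the Door by a local yaw step of Speed times Angle, negated when closing, while AngleProgress accumulates Speed.
; When progress nearly equals AngleMax, it resets and flips the open state.
; Steps ignore delta time, so motion is frame-rate dependent.
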(event `self.ReceiveTick`
  (params (DeltaSeconds :type "Float (single-precision)"))
  (bind _door (`self.Door`))
  (bind _returnvalue (`KismetMathLibrary.MakeRot` 0.0 (* (`self.Speed`) (`self.Angle`))))
  (if (and (`self.DoorChanging`) (not (`KismetMathLibrary.NearlyEqual_FloatFloat` (`self.AngleMax`) (`self.AngleProgress`))))
    (if (not (`self.IsDoorOpened`))
      (`SceneComponent.K2_AddLocalRotation` _door _returnvalue false)
      (else
        (`SceneComponent.K2_AddLocalRotation` _door (`KismetMathLibrary.NegateRotator` _returnvalue) false)))
    (set `self.AngleProgress` (+ (`self.AngleProgress`) (`self.Speed`)))
    (if (`KismetMathLibrary.NearlyEqual_FloatFloat` (`self.AngleMax`) (`self.AngleProgress`))
      (set `self.AngleProgress` 0.0)
      (set `self.DoorChanging` false)
      (set `self.IsDoorOpened` (not (`self.IsDoorOpened`))))))

(event `DoorOrderAction`
  (if (not (`self.DoorChanging`))
    (set `self.DoorChanging` true)
    (set `self.AngleProgress` 0.0)))

(fn `UserConstructionScript`)