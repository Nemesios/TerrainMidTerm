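; Double door held by five locks that opens once the player has collected enough keys.
; CheckForKey compares the character's Collectibles to the last count and hides one live lock per new key, tracked in a struct array built in the Construction Script.
; When no locks remain, DoorOrderAction starts Tick rotating both leaves in opposite directions until AngleMax, then flips the open state, so later calls reverse the swing.
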(event `CheckForKey`
  (params (NewParam :type "/Game/Blueprints/MyCharacter Object Reference"))
  ;[1 1 1] Check Character Keys
  (bind _asmy_character (cast `/Game/Blueprints/MyCharacter` NewParam))
  (set `self.LocksToDelete` (- (`/Game/Blueprints/MyCharacter.Collectibles` _asmy_character) (`self.LastAmountKeys`)))
  (set `self.LastAmountKeys` (`/Game/Blueprints/MyCharacter.Collectibles` _asmy_character))
  (for (_array_element _array_index) (`self.Locks`)
    (bind (_mesh _isalive) (break `/Game/Structure/LockStruct` _array_element))
    (if (and _isalive (> (`self.LocksToDelete`) 0))
      (`SceneComponent.ToggleVisibility` _mesh false)
      (set `self.LocksToDelete` (- (`self.LocksToDelete`) 1))
      (`KismetArrayLibrary.Array_Set` (`self.Locks`) _array_index (make `/Game/Structure/LockStruct` _mesh))))
  (`self.CheckForLocks`))

(event `CheckForLocks`
  ;[1 1 1] Check for number of locks on door
  (if (not (`self.IsDoorOpened`))
    (set `self.DoorUnlocked` true)
    (for _array_element (`self.Locks`)
      (if (`.IsAlive_3_C659439048130B6D3F7248B7FA3AA86A` (break `/Game/Structure/LockStruct` _array_element))
        (set `self.DoorUnlocked` false)))
    (if (`self.DoorUnlocked`)
      (`self.DoorOrderAction`))))

(event `self.ReceiveTick`
  (params (DeltaSeconds :type "Float (single-precision)"))
  (bind _doorright (`self.DoorRight`))
  (bind _doorleft (`self.DoorLeft`))
  (bind _returnvalue (`KismetMathLibrary.MakeRot` 0.0 (* (`self.Speed`) (`self.Angle`))))
  (bind _returnvalue_2 (`KismetMathLibrary.NegateRotator` _returnvalue))
  ;[1 1 1] Open double door
  (if (and (`self.DoorChanging`) (not (`KismetMathLibrary.NearlyEqual_FloatFloat` (`self.AngleMax`) (`self.AngleProgress`))))
    (if (not (`self.IsDoorOpened`))
      (`SceneComponent.K2_AddLocalRotation` _doorright _returnvalue false)
      (`SceneComponent.K2_AddLocalRotation` _doorleft _returnvalue_2 false)
      (else
        (`SceneComponent.K2_AddLocalRotation` _doorright _returnvalue_2 false)
        (`SceneComponent.K2_AddLocalRotation` _doorleft _returnvalue false)))
    (set `self.AngleProgress` (+ (`self.AngleProgress`) (`self.Speed`)))
    (if (`KismetMathLibrary.NearlyEqual_FloatFloat` (`self.AngleMax`) (`self.AngleProgress`))
      (set `self.AngleProgress` 0.0)
      (set `self.DoorChanging` false)
      (set `self.IsDoorOpened` (not (`self.IsDoorOpened`))))))

(event `DoorOrderAction`
  ;[1 1 1] Open double door
  (if (not (`self.DoorChanging`))
    (set `self.DoorChanging` true)
    (set `self.AngleProgress` 0.0)))

(fn `UserConstructionScript`
  (set `self.Locks` (`|MakeArray` (make `/Game/Structure/LockStruct` (`self.Lock1`) true) (make `/Game/Structure/LockStruct` (`self.Lock2`) true) (make `/Game/Structure/LockStruct` (`self.Lock3`) true) (make `/Game/Structure/LockStruct` (`self.Lock4`) true) (make `/Game/Structure/LockStruct` (`self.Lock5`) true))))