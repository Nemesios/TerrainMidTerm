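; LightSwitch is a trigger actor that lights a list of wall sconces when an actor overlaps it.
; Its construction script sets every Blueprint_WallSconce in Lights to zero intensity, so they start dark.
; On overlap, it loops over Lights, sets each sconce to Brightness through MySetIntensity, then calls a Delay inside the loop body.
; Entries that fail the sconce cast print a debug message.
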(event `self.ReceiveActorBeginOverlap`
  (params (OtherActor :type "Actor Object Reference"))
  (for _array_element (`self.Lights`)
    (bind _asblueprint_wall_sconce (cast `/Game/StarterContent/Blueprints/Blueprint_WallSconce` _array_element)
      (:`then`
        (`/Game/StarterContent/Blueprints/Blueprint_WallSconce.MySetIntensity` _asblueprint_wall_sconce (`self.Brightness`))
        (`KismetSystemLibrary.Delay` (`self.Delay`)))
      (:`CastFailed`
        (`KismetSystemLibrary.PrintString` "Cast Fail Event LightSwitch")))))

(fn `UserConstructionScript`
  (for _array_element (`self.Lights`)
    (bind _asblueprint_wall_sconce (cast `/Game/StarterContent/Blueprints/Blueprint_WallSconce` _array_element)
      (:`then`
        (`/Game/StarterContent/Blueprints/Blueprint_WallSconce.MySetIntensity` _asblueprint_wall_sconce 0.0))
      (:`CastFailed`
        (`KismetSystemLibrary.PrintString` "Cast Fail Const LightSwitch")))))